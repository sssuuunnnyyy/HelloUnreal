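; BP_MoveUpDown is a Blueprint that moves its Cube component up and down continuously along its relative Z axis.
; Each Tick adds a fixed relative offset without sweep, and the IsMoveUp flag picks the direction.
; The flag flips when the Cube reaches EndPoint or drops below zero.
; The step ignores delta time, so speed depends on frame rate.
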(event `self.ReceiveTick`
  (params (DeltaSeconds :type "Float (single-precision)"))
  (bind _cube (`self.Cube`))
  (bind (_relativelocation_x _relativelocation_y _relativelocation_z) (`KismetMathLibrary.BreakVector` (`SceneComponent.RelativeLocation` _cube)))
  (bind (_relativelocation_x_2 _relativelocation_y_2 _relativelocation_z_2) (`KismetMathLibrary.BreakVector` (`SceneComponent.RelativeLocation` _cube)))
  (if (`self.IsMoveUp`)
    (`SceneComponent.K2_AddRelativeLocation` _cube (0.0 0.0 5.0) false false)
    (if (>= _relativelocation_z (`self.EndPoint`))
      (set `self.IsMoveUp` false))
    (else
      (`SceneComponent.K2_AddRelativeLocation` (`self.Cube`) (-0.0 0.0 -5.0) false false)
      (if (< _relativelocation_z_2 0.0)
        (set `self.IsMoveUp` true)))))

(fn `UserConstructionScript`)